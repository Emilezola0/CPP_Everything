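; BP_CrossDiagonal is a construction-script actor that builds an X of stone meshes on a square grid in its local XZ plane.
; It loops over a StonesXY-sized grid and adds a Hierarchical Instanced Static Mesh instance wherever a cell lies on either diagonal.
; Spacing comes from the mesh bounds, and a TextRender shows the instance count.
; The Feur edge-check helper is unused, and the event graph is empty.
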(fn `Feur`
  (params (Index :type Integer) (Stone :type Integer))
  (returns (ReturnValue :type Boolean))
  (return (or (== (`local.Index`) 0) (== (- (`local.Stone`) 1) (`local.Index`)))))

(fn `getMeshHalfSize`
  (returns (NewParam :type "Vector Structure"))
  (bind (_returnvalue_origin _returnvalue_boxextent) (`KismetMathLibrary.BreakBoxSphereBounds` (`StaticMesh.GetBounds` (`self.SM_Stone`))))
  (return (- _returnvalue_boxextent _returnvalue_origin)))

(fn `UserConstructionScript`
  (locals (L_Xindex :type Integer) (L_Yindex :type Integer) (L_CurrentMin :type Integer) (L_CurrentMax :type Integer))
  (`InstancedStaticMeshComponent.ClearInstances` (`self.HierarchicalInstancedStaticMesh`))
  (if (and (`KismetSystemLibrary.IsValid` (`self.SM_Stone`)) (> (`self.Stones_XY`) 0))
    (`StaticMeshComponent.SetStaticMesh` (`self.HierarchicalInstancedStaticMesh`) (`self.SM_Stone`))
    (for _index (range (`self.Stones_XY`))
      (set `local.L_Yindex` _index)
      (for _index_2 (range (`self.Stones_XY`))
        (set `local.L_Xindex` _index_2)
        ; Add to Min and Reduce Max each time Y Index increase
        (set `local.L_CurrentMin` (`local.L_Yindex`))
        (set `local.L_CurrentMax` (- (- (`self.Stones_XY`) 1) (`local.L_Yindex`)))
        (if (or (== (`local.L_CurrentMin`) (`local.L_Xindex`)) (== (`local.L_CurrentMax`) (`local.L_Xindex`)))
          (`InstancedStaticMeshComponent.AddInstance` (`self.HierarchicalInstancedStaticMesh`) (`KismetMathLibrary.MakeTransform` (* (* (`self.getMeshHalfSize`) 2.0) (`KismetMathLibrary.MakeVector` (`KismetMathLibrary.Conv_IntToDouble` (`local.L_Xindex`)) 0.0 (`KismetMathLibrary.Conv_IntToDouble` (`local.L_Yindex`))))) false))))
    (`TextRenderComponent.K2_SetText` (`self.TextRender`) (`|FormatText` "{count}" (`InstancedStaticMeshComponent.GetInstanceCount` (`self.HierarchicalInstancedStaticMesh`))))))