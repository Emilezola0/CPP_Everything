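; Wall Blueprint that procedurally builds a grid of stone meshes along local X and Z in the editor-time Construction Script.
; It clears and refills a Hierarchical Instanced Static Mesh component, spacing instances by the mesh's bounding-box size and applying a vertical offset.
; An optional debug toggle shows the Blueprint name and instance count as text components.
; The Event Graph holds no active logic.
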(fn `UserConstructionScript`
  (locals (L_StoneSizeX :type "Float (double-precision)") (L_StoneSizeZ :type "Float (double-precision)" :default 0.0) (L_StoneLocation_X :type "Vector Structure") (L_StoneLocation_Z :type "Vector Structure"))
  (bind (_returnvalue_min _returnvalue_max) (break `Box` (`StaticMesh.GetBoundingBox` (`self.SM_Stone`))))
  (bind (_returnvalue_min_2 _returnvalue_max_2) (break `Box` (`StaticMesh.GetBoundingBox` (`self.SM_Stone`))))
  (bind _returnvalue_x (`KismetMathLibrary.BreakVector` (- _returnvalue_max_2 _returnvalue_min_2)))
  (bind (_returnvalue_x_2 _returnvalue_y _returnvalue_z) (`KismetMathLibrary.BreakVector` (- _returnvalue_max _returnvalue_min)))
  (`InstancedStaticMeshComponent.ClearInstances` (`self.HISM_00`))
  (`StaticMeshComponent.SetStaticMesh` (`self.HISM_00`) (`self.SM_Stone`))
  (if (and (> (`self.Stones_X`) 0) (> (`self.Stones_Z`) 0) (`KismetSystemLibrary.IsValid` (`self.SM_Stone`)))
    (set `local.L_StoneSizeX` _returnvalue_x)
    (set `local.L_StoneSizeZ` _returnvalue_z)
    (for _index (range (`self.Stones_X`))
      (set `local.L_StoneLocation_X` (+ (* _index (`KismetMathLibrary.MakeVector` (`local.L_StoneSizeX`))) (`KismetMathLibrary.MakeVector` 0.0 0.0 (`self.StoneZOffset`))))
      (for _index_2 (range (`self.Stones_Z`))
        (set `local.L_StoneLocation_Z` (* _index_2 (`KismetMathLibrary.MakeVector` 0.0 0.0 (`local.L_StoneSizeZ`))))
        (`InstancedStaticMeshComponent.AddInstance` (`self.HISM_00`) (`KismetMathLibrary.MakeTransform` (+ (`local.L_StoneLocation_Z`) (`local.L_StoneLocation_X`))) false)))
    (`SceneComponent.SetVisibility` (`self.CubeCount`) (`self.RenderText`) false)
    (`SceneComponent.SetVisibility` (`self.Bp_Name`) (`self.RenderText`) false)
    ;[1 1 0 0.15] Debug Only
    (if (`self.RenderText`)
      (`TextRenderComponent.K2_SetText` (`self.CubeCount`) (`KismetTextLibrary.Conv_StringToText` (`KismetStringLibrary.Concat_StrStr` "Cube Count : " (`KismetStringLibrary.Conv_IntToString` (`InstancedStaticMeshComponent.GetInstanceCount` (`self.HISM_00`)))))))))