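; A spline placement Blueprint that lays a row of stone meshes along a spline, each with randomized rotation and scale.
; The construction script rebuilds a single HISM, spacing instances evenly by distance from start to end with a Z offset.
; A seeded random stream adds a random rotation to the spline's and picks scale independently per axis within a range.
; Optional text components show a debug label and instance count.
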(fn `UserConstructionScript`
  (locals (L_StoneLocation :type "Vector Structure") (L_StoneRotation :type "Rotator Structure") (L_StoneScale :type "Vector Structure") (L_InstanceTransform :type "Transform Structure"))
  (set `self.Stream` (`KismetMathLibrary.MakeRandomStream` (`self.Seed`)))
  (`InstancedStaticMeshComponent.ClearInstances` (`self.HISM_00`))
  (`StaticMeshComponent.SetStaticMesh` (`self.HISM_00`) (`self.SM_Stone`))
  (if (> (`self.Stones`) 0)
    (for _index (range (`self.Stones`))
      (bind _returnvalue (* _index (/ (`SplineComponent.GetSplineLength` (`self.Spline`)) (- (`self.Stones`) 1))))
      (set `local.L_StoneLocation` (+ (`SplineComponent.GetLocationAtDistanceAlongSpline` (`self.Spline`) _returnvalue "World") (`KismetMathLibrary.MakeVector` 0.0 0.0 (`self.StoneZOffset`))))
      (set `local.L_StoneRotation` (`KismetMathLibrary.ComposeRotators` (`SplineComponent.GetRotationAtDistanceAlongSpline` (`self.Spline`) _returnvalue "World") (`KismetMathLibrary.RandomRotatorFromStream` (`self.Stream`) true)))
      (set `local.L_StoneScale` (`KismetMathLibrary.MakeVector` (`KismetMathLibrary.RandomFloatInRangeFromStream` (`self.Stream`) (`self.MinScale`) (`self.MaxScale`)) (`KismetMathLibrary.RandomFloatInRangeFromStream` (`self.Stream`) (`self.MinScale`) (`self.MaxScale`)) (`KismetMathLibrary.RandomFloatInRangeFromStream` (`self.Stream`) (`self.MinScale`) (`self.MaxScale`))))
      (set `local.L_InstanceTransform` (`KismetMathLibrary.MakeTransform` (`local.L_StoneLocation`) (`local.L_StoneRotation`) (`local.L_StoneScale`)))
      (`InstancedStaticMeshComponent.AddInstance` (`self.HISM_00`) (`local.L_InstanceTransform`) true)))
  (`SceneComponent.SetVisibility` (`self.CubeCount`) (`self.RenderText`) false)
  (`SceneComponent.SetVisibility` (`self.Bp_Name`) (`self.RenderText`) false)
  ;[1 1 0 0.15] Debug Only
  (if (`self.RenderText`)
    (`TextRenderComponent.K2_SetText` (`self.CubeCount`) (`KismetTextLibrary.Conv_StringToText` (`KismetStringLibrary.Concat_StrStr` "Cube Count : " (`KismetStringLibrary.Conv_IntToString` (`InstancedStaticMeshComponent.GetInstanceCount` (`self.HISM_00`))))))))