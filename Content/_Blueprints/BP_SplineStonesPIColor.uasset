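; Construction-script actor that lines a spline with evenly spaced stone meshes, each given a random hue through per-instance custom data.
; It rebuilds a Hierarchical Instanced Static Mesh on construction, spacing instances from end to end with spline rotation and a Z offset.
; Each hue's RGB fills custom data slots 0–2, intended for the assigned material.
; Optional text components show the instance count and Blueprint name for debugging.
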(fn `UserConstructionScript`
  (locals (L_StoneLocation :type "Vector Structure") (L_StoneRotation :type "Rotator Structure") (L_StoneScale :type "Vector Structure" :default (1.0 1.0 1.0)) (L_InstanceTransform :type "Transform Structure") (L_DynMat :type "MaterialInstanceDynamic Object Reference") (L_Index :type Integer) (L_Color :type "LinearColor Structure"))
  (bind (_r _g _b) (break `LinearColor` (`local.L_Color`)))
  (`InstancedStaticMeshComponent.ClearInstances` (`self.HISM_00`))
  (`StaticMeshComponent.SetStaticMesh` (`self.HISM_00`) (`self.SM_Stone`))
  (`PrimitiveComponent.SetMaterial` (`self.HISM_00`) 0 (`self.PICDMaterial`))
  (if (> (`self.Stones`) 0)
    (for _index (range (`self.Stones`))
      (bind _output_get (set `local.L_Index` _index))
      (bind _returnvalue (* _output_get (/ (`SplineComponent.GetSplineLength` (`self.Spline`)) (- (`self.Stones`) 1))))
      (set `local.L_StoneLocation` (+ (`SplineComponent.GetLocationAtDistanceAlongSpline` (`self.Spline`) _returnvalue "World") (`KismetMathLibrary.MakeVector` 0.0 0.0 (`self.StoneZOffset`))))
      (set `local.L_StoneRotation` (`SplineComponent.GetRotationAtDistanceAlongSpline` (`self.Spline`) _returnvalue "World"))
      (set `local.L_InstanceTransform` (`KismetMathLibrary.MakeTransform` (`local.L_StoneLocation`) (`local.L_StoneRotation`) (`local.L_StoneScale`)))
      (bind _returnvalue_2 (`InstancedStaticMeshComponent.AddInstance` (`self.HISM_00`) (`local.L_InstanceTransform`) true))
      (`KismetMathLibrary.LinearColor_SetRandomHue` (`local.L_Color`))
      (`InstancedStaticMeshComponent.SetCustomDataValue` (`self.HISM_00`) _returnvalue_2 0 _r false)
      (`InstancedStaticMeshComponent.SetCustomDataValue` (`self.HISM_00`) _returnvalue_2 1 _g false)
      (`InstancedStaticMeshComponent.SetCustomDataValue` (`self.HISM_00`) _returnvalue_2 2 _b false)))
  (`SceneComponent.SetVisibility` (`self.CubeCount`) (`self.RenderText`) false)
  (`SceneComponent.SetVisibility` (`self.Bp_Name`) (`self.RenderText`) false)
  ;[1 1 0 0.15] Debug Only
  (if (`self.RenderText`)
    (`TextRenderComponent.K2_SetText` (`self.CubeCount`) (`KismetTextLibrary.Conv_StringToText` (`KismetStringLibrary.Concat_StrStr` "Cube Count : " (`KismetStringLibrary.Conv_IntToString` (`InstancedStaticMeshComponent.GetInstanceCount` (`self.HISM_00`))))))))