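; Procedural pyramid of randomly colored cubes, built in the construction script from a stone mesh, material and layer count.
; Each layer adds a shrinking square grid of HISM instances, centered by a half-stone shift per level and spaced by mesh bounds.
; Each instance gets a random RGB through three custom data floats.
; Two text components above the apex show a configurable label and the cube count.
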(fn `FindTransformForWall`
  (params (NumberOfCube :type Integer) (OffsetZ :type "Float (double-precision)"))
  (returns (ReturnValue :type "Transform Structure"))
  (for _index (range (+ (`local.NumberOfCube`) 1))
    (for _index_2 (range (+ (`local.NumberOfCube`) 1))
      (return (`KismetMathLibrary.MakeTransform` (`KismetMathLibrary.MakeVector` (+ (.x (* _index (`self.getSM_Size`))) (.x (* (* (`KismetSystemLibrary.MakeLiteralDouble` (/ (`local.NumberOfCube`) 2.0)) -1.0) (`self.getSM_Size`)))) (+ (.y (* _index_2 (`self.getSM_Size`))) (.y (* (* (`KismetSystemLibrary.MakeLiteralDouble` (/ (`local.NumberOfCube`) 2.0)) -1.0) (`self.getSM_Size`)))) (`local.OffsetZ`)))))))

(fn `getRandomColor`
  (returns (ReturnValue :type "LinearColor Structure"))
  (return (`KismetMathLibrary.MakeColor` (`KismetMathLibrary.RandomFloatInRange` 0.0 1.0) (`KismetMathLibrary.RandomFloatInRange` 0.0 1.0) (`KismetMathLibrary.RandomFloatInRange` 0.0 1.0))))

(fn `getSM_Size`
  (returns (ReturnValue :type "Vector Structure") (HalfSize :type "Vector Structure"))
  (bind (_returnvalue_origin _returnvalue_boxextent) (`KismetMathLibrary.BreakBoxSphereBounds` (`StaticMesh.GetBounds` (`self.SM_Stone`))))
  (bind _returnvalue (- _returnvalue_boxextent _returnvalue_origin))
  (return (* _returnvalue 2.0) _returnvalue))

(fn `getTopOfThePyramid`
  (returns (ReturnValue :type "Vector Structure"))
  (bind (_returnvalue _halfsize) (`self.getSM_Size`))
  (return (`KismetMathLibrary.MakeVector` (- (.x (/ (* (`self.Stones_Z`) _returnvalue) (2.0 2.0 1.0))) (.x _halfsize)) (- (.y (/ (* (`self.Stones_Z`) _returnvalue) (2.0 2.0 1.0))) (.y _halfsize)) (+ (.z (/ (* (`self.Stones_Z`) _returnvalue) (2.0 2.0 1.0))) (`self.StoneZ_Offset`)))))

(fn `RGB`
  (params (InstanceIndex :type Integer) (linearColor :type "LinearColor Structure"))
  (bind (_linearcolor_r _linearcolor_g _linearcolor_b) (break `LinearColor` (`local.linearColor`)))
  (`InstancedStaticMeshComponent.SetCustomDataValue` (`self.HierarchicalInstancedStaticMesh`) InstanceIndex 0 _linearcolor_r false)
  (`InstancedStaticMeshComponent.SetCustomDataValue` (`self.HierarchicalInstancedStaticMesh`) InstanceIndex 1 _linearcolor_g false)
  (`InstancedStaticMeshComponent.SetCustomDataValue` (`self.HierarchicalInstancedStaticMesh`) InstanceIndex 2 _linearcolor_b false))

(fn `UserConstructionScript`
  (locals (L_HeightIndex :type Integer))
  (bind _returnvalue (- (- (`self.Stones_Z`) (`local.L_HeightIndex`)) 1))
  (`InstancedStaticMeshComponent.ClearInstances` (`self.HierarchicalInstancedStaticMesh`))
  (if (and (`KismetSystemLibrary.IsValid` (`self.SM_Stone`)) (>= (`self.Stones_Z`) 1) (`KismetSystemLibrary.IsValid` (`self.StoneMaterial`)))
    (`SceneComponent.SetVisibility` (`self.NameBP`) (`self.TextRender?`) false)
    (`SceneComponent.SetVisibility` (`self.CountCubes`) (`self.TextRender?`) false)
    (`PrimitiveComponent.SetMaterial` (`self.HierarchicalInstancedStaticMesh`) 0 (`self.StoneMaterial`))
    (`StaticMeshComponent.SetStaticMesh` (`self.HierarchicalInstancedStaticMesh`) (`self.SM_Stone`))
    ; Height
    (for _index (range (`self.Stones_Z`))
      (set `local.L_HeightIndex` _index)
      ; Floor
      (for _index_2 (range (+ _returnvalue 1))
        (for _index_3 (range (+ _returnvalue 1))
          (bind _returnvalue_2 (`InstancedStaticMeshComponent.AddInstance` (`self.HierarchicalInstancedStaticMesh`) (`KismetMathLibrary.MakeTransform` (`KismetMathLibrary.MakeVector` (+ (.x (* _index_2 (`self.getSM_Size`))) (.x (* (`KismetSystemLibrary.MakeLiteralDouble` (/ (`local.L_HeightIndex`) 2.0)) (`self.getSM_Size`)))) (+ (.y (* _index_3 (`self.getSM_Size`))) (.y (* (`KismetSystemLibrary.MakeLiteralDouble` (/ (`local.L_HeightIndex`) 2.0)) (`self.getSM_Size`)))) (+ (.z (* (`local.L_HeightIndex`) (`self.getSM_Size`))) (`self.StoneZ_Offset`)))) false))
          (`self.RGB` _returnvalue_2 (`self.getRandomColor`)))))
    ; Texts
    (`SceneComponent.K2_SetRelativeLocationAndRotation` :`self` (`self.NameBP`) :`NewLocation` (`KismetMathLibrary.MakeVector` (.x (`self.getTopOfThePyramid`)) (.y (`self.getTopOfThePyramid`)) (+ (.z (`self.getTopOfThePyramid`)) 25.0)))
    (`SceneComponent.K2_SetRelativeLocationAndRotation` :`self` (`self.CountCubes`) :`NewLocation` (`self.getTopOfThePyramid`))
    (`TextRenderComponent.K2_SetText` (`self.NameBP`) (`self.TextToShow`))
    (`TextRenderComponent.K2_SetText` (`self.CountCubes`) (`|FormatText` "Cubes Count : {number}" (`InstancedStaticMeshComponent.GetInstanceCount` (`self.HierarchicalInstancedStaticMesh`))))))